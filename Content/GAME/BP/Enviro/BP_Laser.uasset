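; BP_Laser is a laser hazard that knocks the player turtle back on contact.
; The construction script fills LasersArray with LeftSocket01 and one added mesh raised by Step.
; BeginPlay makes each query-only and binds its overlap, which launches BP_PlayerTurtle against its velocity with a random per-axis multiplier.
; The Desactivate event is an empty stub.
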(event Custom|Desactivate)

(event Custom|OnComponentBeginOverlap_Event
  (params (OverlappedComponent :type Primitive%20Component%20Object%20Reference) (OtherActor :type Actor%20Object%20Reference) (OtherComp :type Primitive%20Component%20Object%20Reference) (OtherBodyIndex :type Integer) (bFromSweep :type Boolean) (SweepResult :type Hit%20Result%20Structure%20%28by%20ref%29))
  (CallFunction|Overlap OtherActor))

(event Custom|Overlap
  (params (NewParam :type Actor%20Object%20Reference))
  (bind _returnvalue (Math|Random|RandomFloatinRange 1.0 5.0))
  (bind _asbp_player_turtle (Utilities|Casting|CastToBP_PlayerTurtle NewParam))
  (Character|LaunchCharacter _asbp_player_turtle (Math|Vector|MakeVector (* (.x (Math|Vector|NegateVector (Transformation|GetVelocity _asbp_player_turtle))) _returnvalue) (* (.y (Math|Vector|NegateVector (Transformation|GetVelocity _asbp_player_turtle))) _returnvalue) (* (.z (Math|Vector|NegateVector (Transformation|GetVelocity _asbp_player_turtle))) _returnvalue)) true true))

(event EventBeginPlay
  (for _array_element (Variables|Default|GetLasersArray)
    (Collision|SetCollisionEnabled _array_element "QueryOnly")
    (Collision|AssignOnComponentBeginOverlap _array_element (delegate Custom|OnComponentBeginOverlap_Event))))

(fn ConstructionScript
  (bind _leftsocket01 (Variables|Default|GetLeftSocket01))
  (bind _lasersarray (Variables|Default|GetLasersArray))
  (bind _relativelocation (Variables|/Script/Engine.SceneComponent|GetRelativeLocation _leftsocket01))
  (bind (_x _y _z) (Class|KismetMathLibrary|BreakVector3f _relativelocation))
  (Utilities|Array|Clear _lasersarray)
  (Utilities|Array|Add _lasersarray (Variables|Default|GetLeftSocket01))
  (bind _returnvalue (AddComponent|AddStaticMeshComponent false (Math|Transform|MakeTransform (Math|Vector|MakeVector _x _y (+ _z (Variables|Default|GetStep))) "0, 0, 0" "0.062500,0.062500,0.062500")))
  (bind _output_get (Variables|Default|SetActualLaser _returnvalue))
  (Utilities|Array|Add (Variables|Default|GetLasersArray) _output_get))