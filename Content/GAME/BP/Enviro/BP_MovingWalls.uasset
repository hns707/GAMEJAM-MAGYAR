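; BP_MovingWalls is an environment actor: a wall that moves between a bottom and a top marker.
; The construction script scales the wall by a Length variable and sets the Top marker's height from Hauteur.
; On BeginPlay it caches both markers' world positions and plays the Move timeline, whose HautBas track lerps the root between them without sweep.
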(event EventBeginPlay
  (Variables|Default|SetBotPos (Transformation|GetWorldLocation (Variables|Default|GetBot)))
  (Variables|Default|SetTopPos (Transformation|GetWorldLocation (Variables|Default|GetTop)))
  (bind _haut_bas (Timeline|Move Play)
    (:Update
      (Transformation|SetWorldLocation (Variables|Default|GetDefaultSceneRoot) (Math|Vector|Lerp(Vector) (Variables|Default|GetBotPos) (Variables|Default|GetTopPos) _haut_bas) false false))))

(fn ConstructionScript
  (bind _top (Variables|Default|GetTop))
  (bind _relativelocation (Variables|/Script/Engine.SceneComponent|GetRelativeLocation _top))
  (Transformation|SetWorldScale3D (Variables|Default|GetWall) (Math|Vector|MakeVector (Variables|Default|GetLength) 0.1 1.0))
  (Transformation|SetRelativeLocation _top (Math|Vector|MakeVector (.x _relativelocation) (.y _relativelocation) (Variables|Default|GetHauteur)) false false))