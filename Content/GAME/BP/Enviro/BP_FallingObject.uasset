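; BP_FallingObject is an environment hazard whose Falling component drops when something overlaps its trigger Box.
; The construction script line-traces down from Falling by LineTraceLength and moves the Box to the impact point, placing the trigger beneath the object.
; Overlap enables physics simulation on Falling.
; On hit, it runs a debug-drawn sphere trace at the impact point, leaves the result unused, and destroys the actor.
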(event OnComponentBeginOverlap(Box)
  (params (OverlappedComponent :type Primitive%20Component%20Object%20Reference) (OtherActor :type Actor%20Object%20Reference) (OtherComp :type Primitive%20Component%20Object%20Reference) (OtherBodyIndex :type Integer) (bFromSweep :type Boolean) (SweepResult :type Hit%20Result%20Structure%20%28by%20ref%29))
  (Development|PrintString "PlayerDetected ")
  (Physics|SetSimulatePhysics (Variables|Default|GetFalling) true))

(event OnComponentHit(Falling)
  (params (HitComponent :type Primitive%20Component%20Object%20Reference) (OtherActor :type Actor%20Object%20Reference) (OtherComp :type Primitive%20Component%20Object%20Reference) (NormalImpulse :type Vector :default "0, 0, 0") (Hit :type Hit%20Result%20Structure%20%28by%20ref%29))
  (bind _impactpoint (Collision|BreakHitResult Hit))
  (Development|PrintString "boom")
  (Collision|SphereTraceByChannel _impactpoint _impactpoint 1e+02 "TraceTypeQuery1" false 0 "Persistent")
  (Actor|DestroyActor))

(fn ConstructionScript
  (bind _falling (Variables|Default|GetFalling))
  (bind _returnvalue (Transformation|GetWorldLocation _falling))
  (bind (_x _y _z) (Class|KismetMathLibrary|BreakVector3f _returnvalue))
  (bind (_outhit _returnvalue_2) (Collision|LineTraceByChannel _returnvalue (Math|Vector|MakeVector _x _y (- _z (Variables|Default|GetLineTraceLength))) "TraceTypeQuery1" false 0 "ForOneFrame"))
  (if _returnvalue_2
    (Transformation|SetWorldLocation (Variables|Default|GetBox) (.ImpactPoint (Collision|BreakHitResult _outhit)) false false)))