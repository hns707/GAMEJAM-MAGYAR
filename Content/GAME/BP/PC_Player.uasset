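; Player controller that drives a turtle with four grappling arms used as a slingshot, and cycles level cameras with a UI label.
; Front and back inputs line-trace arm pairs from socket rotations and store anchor points.
; While anchored, Tract pulls the turtle away from the anchors under altered gravity; releasing launches it along the mesh's right vector, scaled by displacement.
; Otherwise input rotates, pitches or jumps the turtle.
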(event Custom|ManageSpring
  (params (Hold :type Boolean) (PowerInverter :type Float%20%28double-precision%29))
  (bind _playerref_tortue (Variables|Default|GetPlayerRef_Tortue))
  ;[1 1 1] SpringManagement
  (Utilities|FlowControl|Sequence
    (:then_0
      (if (not (Variables|Default|GetChargeSpring))
        (Utilities|FlowControl|DoOnce false :!label _label
          (:Completed
            (Variables|Default|SetChargeSpring true)
            (Variables|Default|SetPositionBeforeRelease (Transformation|GetActorLocation (Variables|Default|GetPlayerRef_Tortue)))))
        (else
          (CallFunction|StopGravity))))
    (:then_1
      (if (and (Variables|Default|GetChargeSpring) (not Hold))
        (Utilities|FlowControl|DelayUntilNextTick)
        (Variables|Default|SetChargeSpring false)
        (Default|ActionVelocity _playerref_tortue (* (Math|Vector|GetRightVector (Variables|/Script/Engine.Character|GetMesh (Variables|Default|GetPlayerRef_Tortue))) (* (Math|Float|Clamp(Float) (Math|Vector|Distance(Vector) (Variables|Default|GetPositionBeforeRelease) (Transformation|GetActorLocation _playerref_tortue)) 0.0 1e+03) PowerInverter)) true true)
        (Variables|/Script/Engine.CharacterMovementComponent|SetGravityScale (Variables|/Script/Engine.Character|GetCharacterMovement (Variables|Default|GetPlayerRef_Tortue)) 1.0)
        (goto _label Reset)))))

(event Custom|StopGravity
  (bind _returnvalue (Input|EnhancedActionValues|GetIA_ACFront))
  (bind _returnvalue_2 (Input|EnhancedActionValues|GetIA_ACBack))
  (bind _playerref_tortue (Variables|Default|GetPlayerRef_Tortue))
  (bind _returnvalue_3 (and _returnvalue _returnvalue_2))
  (bind _charactermovement (Variables|/Script/Engine.Character|GetCharacterMovement _playerref_tortue))
  ;[1 1 1] SpringManagement
  (Utilities|FlowControl|DelayUntilNextTick)
  (Variables|/Script/Engine.CharacterMovementComponent|SetGravityScale _charactermovement (Math|Float|SelectFloat 0.0 0.6 _returnvalue_3))
  (if _returnvalue_3
    (Components|Movement|StopMovementImmediately _charactermovement)))

(event Input|EnhancedActionEvents|EnhancedInputActionIA_Rotate
  (params (ActionValue :type Float%20%28double-precision%29) (ElapsedSeconds :type Float%20%28double-precision%29) (TriggeredSeconds :type Float%20%28double-precision%29) (InputAction :type Input%20Action%20Object%20Reference :default "/Game/GAME/INPUTS/Actions/IA_Rotate.IA_Rotate"))
  ;[1 1 1] Rotate/Jump
  (:Triggered
    (if (not (Variables|Default|GetChargeSpring))
      (Default|ActionRotate (Variables|Default|GetPlayerRef_Tortue) ActionValue))))

(event Input|EnhancedActionEvents|EnhancedInputActionIA_Jump
  (params (ActionValue :type Boolean) (ElapsedSeconds :type Float%20%28double-precision%29) (TriggeredSeconds :type Float%20%28double-precision%29) (InputAction :type Input%20Action%20Object%20Reference :default "/Game/GAME/INPUTS/Actions/IA_Jump.IA_Jump"))
  (bind _playerref_tortue (Variables|Default|GetPlayerRef_Tortue))
  ;[1 1 1] Rotate/Jump
  (:Completed
    (if (not (AI|Components|NavMovement|IsFalling (Variables|/Script/Engine.Character|GetCharacterMovement _playerref_tortue)))
      (Default|ActionVelocity _playerref_tortue "0.000000,0.000000,900.000000" false true))))

(event Input|EnhancedActionEvents|EnhancedInputActionIA_CameraSwap
  (params (ActionValue :type Float%20%28double-precision%29) (ElapsedSeconds :type Float%20%28double-precision%29) (TriggeredSeconds :type Float%20%28double-precision%29) (InputAction :type Input%20Action%20Object%20Reference :default "/Game/GAME/INPUTS/Actions/IA_CameraSwap.IA_CameraSwap"))
  (:Started
    (if (> ActionValue 0.0)
      (if (< (Variables|Default|GetIndexOfCam) (- (Utilities|Array|Length (Variables|Default|GetArrayOfCams)) 1))
        (bind _output_get (Variables|Default|SetIndexOfCam (+ (Variables|Default|GetIndexOfCam) 1)))
        (CallFunction|ChangeCamera _output_get)
        (else
          (bind _output_get_2 (Variables|Default|SetIndexOfCam 0))
          (CallFunction|ChangeCamera _output_get_2)))
      (elif (> (Variables|Default|GetIndexOfCam) 0)
        (bind _output_get_3 (Variables|Default|SetIndexOfCam (- (Variables|Default|GetIndexOfCam) 1)))
        (CallFunction|ChangeCamera _output_get_3)
        (else
          (bind _output_get_4 (Variables|Default|SetIndexOfCam (- (Utilities|Array|Length (Variables|Default|GetArrayOfCams)) 1)))
          (CallFunction|ChangeCamera _output_get_4))))))

(event Input|EnhancedActionEvents|EnhancedInputActionIA_AC_Tract
  (params (ActionValue :type Float%20%28double-precision%29) (ElapsedSeconds :type Float%20%28double-precision%29) (TriggeredSeconds :type Float%20%28double-precision%29) (InputAction :type Input%20Action%20Object%20Reference :default "/Game/GAME/INPUTS/Actions/IA_AC_Tract.IA_AC_Tract"))
  (bind _returnvalue (Math|Float|Clamp(Float) ActionValue))
  (bind _playerref_tortue (Variables|Default|GetPlayerRef_Tortue))
  (bind _returnvalue_2 (* _returnvalue 3e+02))
  (bind (_outvelocity _releasevector) (CallFunction|GetVelocitybyArmPoints _returnvalue_2))
  ;[1 1 1] Tract
  (:Triggered
    (if (Variables|Default|GetChargeSpring)
      (if (< (Math|Vector|Distance(Vector) (Variables|Default|GetPositionBeforeRelease) (Transformation|GetActorLocation (Variables|Default|GetPlayerRef_Tortue))) 1e+03)
        (Default|ActionVelocity _playerref_tortue _outvelocity true true)
        (Variables|Default|SetLastStoredDirection _releasevector))
      (else
        (Default|ActionPitch _playerref_tortue ActionValue false))))
  (:Completed
    (CallFunction|StopGravity)))

(event Input|EnhancedActionEvents|EnhancedInputActionIA_ACFront
  (params (ActionValue :type Boolean) (ElapsedSeconds :type Float%20%28double-precision%29) (TriggeredSeconds :type Float%20%28double-precision%29) (InputAction :type Input%20Action%20Object%20Reference :default "/Game/GAME/INPUTS/Actions/IA_ACFront.IA_ACFront"))
  (bind _distance (Variables|Default|GetDistance))
  ;[1 1 1] Comment
  (:Started
    (bind (_hit _impactpoint _arm) (CallFunction|TraceArmPath "NewEnumerator0" _distance))
    (bind (_hit_2 _impactpoint_2 _arm_2) (CallFunction|TraceArmPath "NewEnumerator1" _distance))
    (Default|ActionMoveArm (Variables|Default|GetPlayerRef_Tortue) _arm _impactpoint _arm_2 _impactpoint_2 false)
    (CallFunction|UpdateArmPoint _arm _impactpoint)
    (CallFunction|UpdateArmPoint _arm_2 _impactpoint_2)
    (CallFunction|ManageSpring ActionValue 1e+01 :!label _label))
  (:Completed
    (Default|ActionMoveArm (Variables|Default|GetPlayerRef_Tortue) "NewEnumerator0" "0, 0, 0" "NewEnumerator1" "0, 0, 0" true)
    (CallFunction|UpdateArmPoint "NewEnumerator0" "0, 0, 0")
    (CallFunction|UpdateArmPoint "NewEnumerator1" "0, 0, 0")
    (goto _label)))

(event Input|EnhancedActionEvents|EnhancedInputActionIA_ACBack
  (params (ActionValue :type Boolean) (ElapsedSeconds :type Float%20%28double-precision%29) (TriggeredSeconds :type Float%20%28double-precision%29) (InputAction :type Input%20Action%20Object%20Reference :default "/Game/GAME/INPUTS/Actions/IA_ACBack.IA_ACBack"))
  (bind _distance (Variables|Default|GetDistance))
  ;[1 1 1] Comment
  (:Started
    (bind (_hit _impactpoint _arm) (CallFunction|TraceArmPath "NewEnumerator2" _distance))
    (bind (_hit_2 _impactpoint_2 _arm_2) (CallFunction|TraceArmPath "NewEnumerator3" _distance))
    (Default|ActionMoveArm (Variables|Default|GetPlayerRef_Tortue) _arm _impactpoint _arm_2 _impactpoint_2 false)
    (CallFunction|UpdateArmPoint _arm _impactpoint)
    (CallFunction|UpdateArmPoint _arm_2 _impactpoint_2)
    (CallFunction|ManageSpring ActionValue 1e+01 :!label _label))
  (:Completed
    (Default|ActionMoveArm (Variables|Default|GetPlayerRef_Tortue) "NewEnumerator2" "0, 0, 0" "NewEnumerator3" "0, 0, 0" true)
    (CallFunction|UpdateArmPoint "NewEnumerator2" "0, 0, 0")
    (CallFunction|UpdateArmPoint "NewEnumerator3" "0, 0, 0")
    (goto _label)))

(event EventBeginPlay
  ;[0.3538 0.4651 0.5365] BeginPlay
  (bind _returnvalue (Actor|GetActorOfClass "/Game/GAME/BP/BP_CameraMaster.BP_CameraMaster_C"))
  (for _array_element (Variables|/Game/GAME/BP/BP_CameraMaster.BP_CameraMaster_C|GetArrayOfCamera _returnvalue)
    (Utilities|Array|AddUnique (Variables|Default|GetArrayOfCams) _array_element))
  (Input|AddMappingContext (PlayerController|LocalPlayerSubsystems|GetEnhancedInputLocalPlayerSubsystem) "/Game/GAME/INPUTS/IMC_Player.IMC_Player" 0 "(bIgnoreAllPressedKeysUntilRelease=True,bForceImmediately=False)")
  (bind _returnvalue_2 (Actor|GetActorOfClass "/Game/GAME/BP/BP_PlayerTurtle.BP_PlayerTurtle_C"))
  (Variables|Default|SetPlayerRef_Tortue _returnvalue_2)
  (bind _returnvalue_3 (UserInterface|CreateWidget "/Game/GAME/Widget/WG_Interface.WG_Interface_C"))
  (bind _output_get (Variables|Default|SetWGInterfaceRef _returnvalue_3))
  (UserInterface|Viewport|AddtoViewport _output_get 0)
  (CallFunction|ChangeCamera))

(fn ConstructionScript)

(fn TraceArmPath
  (params (SelectedArm :type E_Arms%20Enum :default "NewEnumerator0") (Distance :type Float%20%28double-precision%29))
  (bind _playerref_tortue (Variables|Default|GetPlayerRef_Tortue))
  (bind _returnvalue (Transformation|GetActorLocation _playerref_tortue))
  (bind (_outhit _returnvalue_2) (Collision|LineTraceByChannel _returnvalue (+ _returnvalue (* (Math|Vector|GetForwardVector (Transformation|GetSocketRotation (Variables|/Script/Engine.Character|GetMesh _playerref_tortue) (Utilities|String|StringToName (Utilities|String|EnumtoString SelectedArm)))) Distance)) "TraceTypeQuery1" false 0 "None" true "(R=1.000000,G=0.000000,B=0.000000,A=1.000000)" "(R=0.000000,G=1.000000,B=0.000000,A=1.000000)" 2.0))
  (return _returnvalue_2 (.ImpactPoint (Collision|BreakHitResult _outhit)) SelectedArm))

(fn UpdateArmPoint
  (params (Arm :type E_Arms%20Enum :default "NewEnumerator0") (Point :type Vector))
  (Utilities|Array|SetArrayElem (Variables|Default|GetConnectedArmPoints) (Utilities|Select :Index Arm :NewEnumerator0 0 :NewEnumerator1 1 :NewEnumerator2 2 :NewEnumerator3 3) Point))

(fn GetArmPoint
  (params (Arm :type E_Arms%20Enum :default "NewEnumerator0"))
  (bind _returnvalue (Utilities|Select :Index Arm :NewEnumerator0 0 :NewEnumerator1 1 :NewEnumerator2 2 :NewEnumerator3 3))
  (bind _connectedarmpoints (Variables|Default|GetConnectedArmPoints))
  (bind _output (Utilities|Array|Get(acopy) _connectedarmpoints _returnvalue))
  (return _output (Math|Vector|Distance(Vector) _output (Transformation|GetActorLocation (Variables|Default|GetPlayerRef_Tortue)))))

(fn GetVelocitybyArmPoints
  (params (BaseForce :type Float%20%28single-precision%29))
  (bind _point (CallFunction|GetArmPoint "NewEnumerator3"))
  (bind _point_2 (CallFunction|GetArmPoint "NewEnumerator0"))
  (bind _point_3 (CallFunction|GetArmPoint "NewEnumerator2"))
  (bind _point_4 (CallFunction|GetArmPoint "NewEnumerator1"))
  (bind _playerref_tortue (Variables|Default|GetPlayerRef_Tortue))
  (bind _playerref_tortue_2 (Variables|Default|GetPlayerRef_Tortue))
  (bind _playerref_tortue_3 (Variables|Default|GetPlayerRef_Tortue))
  (bind _playerref_tortue_4 (Variables|Default|GetPlayerRef_Tortue))
  (bind _returnvalue (Transformation|GetActorLocation _playerref_tortue))
  (bind _returnvalue_2 (Transformation|GetActorLocation _playerref_tortue_2))
  (bind _returnvalue_3 (Transformation|GetActorLocation _playerref_tortue_3))
  (bind _returnvalue_4 (Transformation|GetActorLocation _playerref_tortue_4))
  (bind _returnvalue_5 (Utilities|Operators|EqualEqual :A _point :ErrorTolerance 0.1))
  (bind _returnvalue_6 (Utilities|Operators|EqualEqual :A _point_2 :ErrorTolerance 0.1))
  (bind _returnvalue_7 (Utilities|Operators|EqualEqual :A _point_4 :ErrorTolerance 0.1))
  (bind _returnvalue_8 (Utilities|Operators|EqualEqual :A _point_3 :ErrorTolerance 0.1))
  (bind _returnvalue_9 (Math|Vector|SelectVector _returnvalue _point _returnvalue_5))
  (bind _returnvalue_10 (Math|Vector|SelectVector _returnvalue_2 _point_2 _returnvalue_6))
  (bind _returnvalue_11 (Math|Vector|SelectVector _returnvalue_3 _point_4 _returnvalue_7))
  (bind _returnvalue_12 (Math|Vector|SelectVector _returnvalue_4 _point_3 _returnvalue_8))
  (bind _returnvalue_13 (Math|Vector|GetUnitDirection(Vector) _returnvalue _returnvalue_9))
  (bind _returnvalue_14 (Math|Vector|GetUnitDirection(Vector) _returnvalue_2 _returnvalue_10))
  (bind _returnvalue_15 (Math|Vector|GetUnitDirection(Vector) _returnvalue_3 _returnvalue_11))
  (bind _returnvalue_16 (Math|Vector|GetUnitDirection(Vector) _returnvalue_4 _returnvalue_12))
  (bind _returnvalue_17 (+ _returnvalue_14 _returnvalue_15 _returnvalue_16 _returnvalue_13))
  (return (* (* _returnvalue_17 BaseForce) -1.0) _returnvalue_17))

(fn ChangeCamera
  (params (Index :type Integer))
  (bind _arrayofcams (Variables|Default|GetArrayOfCams))
  (bind _output (Utilities|Array|Get(acopy) _arrayofcams Index))
  (Game|Player|SetViewTargetwithBlend _output 0.0 "VTBlend_Linear" 0.0 false)
  (Default|ChangeCam (Variables|Default|GetWGInterfaceRef) (Utilities|Text|ToText(String) (Utilities|String|Append (Utilities|GetDisplayName _output) ""))))