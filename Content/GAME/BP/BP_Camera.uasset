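; BP_Camera is a switchable world camera that tracks the player turtle and is destroyed when the turtle touches it.
; Each Tick it rotates the camera component to look at the turtle.
; On sphere overlap, it shows a dynamic M_NoiseEffect post-process, waits, calls PC_Player's ChangeCamera if it is the active view, then removes itself from ArrayOfCams and destroys itself.
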(event OnComponentBeginOverlap(SphereCollision)
  (params (OverlappedComponent :type Primitive%20Component%20Object%20Reference) (OtherActor :type Actor%20Object%20Reference) (OtherComp :type Primitive%20Component%20Object%20Reference) (OtherBodyIndex :type Integer) (bFromSweep :type Boolean) (SweepResult :type Hit%20Result%20Structure%20%28by%20ref%29))
  (bind _self self)
  (bind _playercontrollerref (Variables|Default|GetPlayerControllerRef))
  (bind _arrayofcams (Variables|/Game/GAME/BP/PC_Player.PC_Player_C|GetArrayOfCams _playercontrollerref))
  (bind _returnvalue (Utilities|Array|FindItem _arrayofcams _self))
  (Utilities|Casting|CastToBP_PlayerTurtle OtherActor)
  (Rendering|Material|SetScalarParameterValue (Variables|Default|GetNeigeRef) "Opacity" 1.0 :!class /Script/Engine.MaterialInstanceDynamic)
  (Utilities|FlowControl|Delay 2.0)
  (if (== (Variables|/Game/GAME/BP/PC_Player.PC_Player_C|GetIndexOfCam (Variables|Default|GetPlayerControllerRef)) _returnvalue)
    (Default|ChangeCamera (Variables|Default|GetPlayerControllerRef))
    (Utilities|FlowControl|Delay 0.2))
  (Utilities|Array|RemoveIndex (Variables|/Game/GAME/BP/PC_Player.PC_Player_C|GetArrayOfCams (Variables|Default|GetPlayerControllerRef)) _returnvalue)
  (Actor|DestroyActor))

(event EventTick
  (params (DeltaSeconds :type Float%20%28single-precision%29))
  (bind _newvar (Variables|Default|GetNewVar))
  (Utilities|IsValid _newvar
    (:Is%20Valid
      (Transformation|SetWorldRotation (Variables|Default|GetCamera) (Math|Rotator|FindLookatRotation (Transformation|GetActorLocation) (Transformation|GetActorLocation _newvar)) false false))))

(event EventBeginPlay
  (Utilities|FlowControl|Sequence
    (:then_0
      (bind _returnvalue (Actor|GetActorOfClass "/Game/GAME/BP/BP_PlayerTurtle.BP_PlayerTurtle_C"))
      (Variables|Default|SetNewVar _returnvalue)
      (bind _returnvalue_2 (Actor|GetActorOfClass "/Game/GAME/BP/PC_Player.PC_Player_C"))
      (Variables|Default|SetPlayerControllerRef _returnvalue_2))
    (:then_1
      (bind _returnvalue_3 (Rendering|Material|CreateDynamicMaterialInstance "/Game/GAME/MATERIALS/M_NoiseEffect.M_NoiseEffect" "None" "None" :!class /Script/Engine.KismetMaterialLibrary))
      (bind _output_get (Variables|Default|SetNeigeRef _returnvalue_3))
      (Utilities|Array|Insert (Utilities|Struct|BreakWeightedBlendables (Utilities|Struct|BreakPostProcessSettings (Variables|/Script/Engine.CameraComponent|GetPostProcessSettings (Variables|Default|GetCamera)))) (Utilities|Struct|MakeWeightedBlendable 1.0 _output_get)))))

(fn ConstructionScript)