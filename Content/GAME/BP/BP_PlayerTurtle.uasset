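; Player turtle Character that exposes actions for yaw, mid-air flipping, launching and reaching both arms toward target positions.
; Arm moves run two timelines with distance-scaled play rates, feeding interpolated positions and blend toggles to the APB_RealTurtle anim instance.
; Pitch rotates only the mesh while falling and resets on a grounded capsule hit; Tick caps velocity.
; The physical animation setup is left unconnected.
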(event OnComponentHit(CapsuleComponent)
  (params (HitComponent :type Primitive%20Component%20Object%20Reference) (OtherActor :type Actor%20Object%20Reference) (OtherComp :type Primitive%20Component%20Object%20Reference) (NormalImpulse :type Vector :default "0, 0, 0") (Hit :type Hit%20Result%20Structure%20%28by%20ref%29))
  (if (not (AI|Components|NavMovement|IsFalling (Variables|Character|GetCharacterMovement)))
    (CallFunction|ActionPitch 0.0 true)))

(event Custom|Action_Rotate
  (params (Val :type Float%20%28single-precision%29))
  (Pawn|Input|AddControllerYawInput Val))

(event Custom|Action_Velocity
  (params (LaunchVelocity :type Vector) (bXYOverride :type Boolean) (bZOverride :type Boolean))
  (Character|LaunchCharacter LaunchVelocity bXYOverride bZOverride))

(event Custom|Action_MoveArm
  (params (ArmLeft :type E_Arms%20Enum :default "NewEnumerator0") (PositionLeft :type Vector) (ArmRight :type E_Arms%20Enum :default "NewEnumerator0") (PositionRight :type Vector) (Reset :type Boolean))
  (bind _returnvalue (Transformation|GetActorLocation))
  (bind (_l _r) (CallFunction|PlayratebyDistance PositionLeft PositionRight))
  (bind _abpref (Variables|Default|GetAbpRef))
  (bind _abpref_2 (Variables|Default|GetAbpRef))
  (if (not Reset)
    (Components|Timeline|SetPlayRate (Variables|Default|GetArmTravel) _l)
    (Components|Timeline|SetPlayRate (Variables|Default|GetArmTravelBis) _r)
    (Default|MoveArmAlpha _abpref ArmLeft true)
    (Default|MoveArmAlpha _abpref ArmRight true)
    (Utilities|FlowControl|Sequence
      (:then_0
        (bind _alpha (Timeline|ArmTravel PlayFromStart)
          (:Update
            (Default|MoveArmOffset _abpref_2 ArmLeft (Math|Vector|Lerp(Vector) _returnvalue PositionLeft _alpha)))))
      (:then_1
        (bind _alpha_2 (Timeline|ArmTravelBis PlayFromStart)
          (:Update
            (Default|MoveArmOffset _abpref_2 ArmRight (Math|Vector|Lerp(Vector) _returnvalue PositionRight _alpha_2))))))
    (else
      (Default|MoveArmOffset _abpref ArmLeft PositionLeft)
      (Default|MoveArmOffset _abpref ArmRight PositionRight)
      (Default|MoveArmAlpha _abpref ArmLeft false)
      (Default|MoveArmAlpha _abpref ArmRight false))))

(event Custom|Action_Pitch
  (params (Delta%20Rotation%20Y%20%28Pitch%29 :type Float%20%28single-precision%29) (Reset :type Boolean))
  (bind _mesh (Variables|Character|GetMesh))
  (if (not Reset)
    (if (AI|Components|NavMovement|IsFalling (Variables|Character|GetCharacterMovement))
      (Transformation|AddRelativeRotation _mesh (Math|Rotator|MakeRotator (* Delta%20Rotation%20Y%20%28Pitch%29 -1.0) 0.0 0.0) false false))
    (else
      (Transformation|SetRelativeRotation _mesh "0.000000,-90.000000,0.000000" false false))))

(event EventBeginPlay
  (Utilities|FlowControl|Sequence
    (:then_0
      (bind _asapb_real_turtle (Utilities|Casting|CastToAPB_RealTurtle (Components|SkeletalMesh|GetAnimInstance (Variables|Character|GetMesh))))
      (Variables|Default|SetAbpRef _asapb_real_turtle))))

(event EventTick
  (params (DeltaSeconds :type Float%20%28single-precision%29))
  (bind _charactermovement (Variables|Character|GetCharacterMovement))
  (Variables|/Script/Engine.MovementComponent|SetVelocity _charactermovement (Math|Vector|ClampVectorSize (Variables|/Script/Engine.MovementComponent|GetVelocity _charactermovement) 0.0 2e+03)))

(fn ConstructionScript)

(fn PlayratebyDistance
  (params (Left :type Vector) (Right :type Vector))
  (bind _returnvalue (Transformation|GetActorLocation))
  (return (Math|Float|MapRangeClamped (Math|Vector|Distance(Vector) Left _returnvalue) 0.0 5e+03 1.0 4.0) (Math|Float|MapRangeClamped (Math|Vector|Distance(Vector) Right _returnvalue) 0.0 5e+03 1.0 4.0)))